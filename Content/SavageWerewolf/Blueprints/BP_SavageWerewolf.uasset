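; BP_SavageWerewolf is a modular werewolf with fur, normal and torn suit variants built from separate skeletal mesh parts.
; The construction script makes the shirt, pant and body fur parts follow the main Mesh through leader pose, so they share its animation.
; On BeginPlay, each suit group applies its Visible setting and propagates it to child components.
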(event EventBeginPlay
  (bind _fur_suit (Variables|Default|GetFur_Suit))
  (bind _normal_suit (Variables|Default|GetNormal_Suit))
  (bind _torn_suit (Variables|Default|GetTorn_Suit))
  (Rendering|SetVisibility _fur_suit (Variables|/Script/Engine.SceneComponent|GetbVisible _fur_suit) true)
  (Rendering|SetVisibility _normal_suit (Variables|/Script/Engine.SceneComponent|GetbVisible _normal_suit) true)
  (Rendering|SetVisibility _torn_suit (Variables|/Script/Engine.SceneComponent|GetbVisible _torn_suit) true))

(fn ConstructionScript
  (Components|SkinnedMesh|SetLeaderPoseComponent (Variables|Default|GetSK_Shirt_Fur) (Variables|Character|GetMesh) false false))