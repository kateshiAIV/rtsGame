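; Actor component, by its name and path the stat system for an RTS game, that provides lookup of named attributes.
; GetAttributeRef linearly searches the Attributes array by name and returns the matching entry and index.
; GetAttributeValue uses that lookup to select the default, bonus, total, current or max experience field, with -1 for None.
; ModifyAttribute is an empty stub, and the event graph holds no logic.
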(event EventBeginPlay)

(fn GetAttributeRef
  (params (Attribute :type E_AttributeList%20Enum :default "NewEnumerator0"))
  (for (_array_element _array_index) (Utilities|Struct|BreakS_PlayerAttributes (Variables|Default|GetAttributes))
    (LocalVariables|SetAttributeValueLocal _array_element)
    (LocalVariables|SetAttributeIndexLocal _array_index)
    (if (Utilities|Enum|Equal(Enum) Attribute (Utilities|Struct|BreakS_SingleAttribute _array_element))
      (return (LocalVariables|GetAttributeValueLocal) (LocalVariables|GetAttributeIndexLocal)))))

(fn GetAttributeValue
  (params (Type :type E_StatType%20Enum :default "NewEnumerator0") (Attribute :type E_AttributeList%20Enum :default "NewEnumerator0"))
  (bind _attributevalue (CallFunction|GetAttributeRef Attribute))
  (bind (_default _bonus _total _currentexp _maxexp) (Utilities|Struct|BreakS_SingleAttribute _attributevalue))
  (return (Utilities|Select :Index Type :NewEnumerator0 -1.0 :NewEnumerator1 _default :NewEnumerator2 _bonus :NewEnumerator3 _total :NewEnumerator4 _currentexp :NewEnumerator5 _maxexp)))

(fn ModifyAttribute)