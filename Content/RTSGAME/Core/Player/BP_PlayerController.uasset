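; RTS player controller that handles camera input, unit selection and orders, and the main UI.
; Enhanced Input and mouse axes drive the camera pawn's movement component for movement, zoom, edge scrolling and gated panning.
; Left mouse drives HUD marquee selection, while right-click moves and stance events message the HUD's selected units.
; It creates the main widget, triggers staggered unit icon creation, and relays date and game speed between UI, GameState and camera.
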(event Input|EnhancedActionEvents|EnhancedInputActionIA_MoveForward
  (params (ActionValue :type Float%20%28double-precision%29) (ElapsedSeconds :type Float%20%28double-precision%29) (TriggeredSeconds :type Float%20%28double-precision%29) (InputAction :type Input%20Action%20Object%20Reference :default "/Game/RTSGAME/Core/Settings/Input/Actions/IA_MoveForward.IA_MoveForward"))
  ;[1 1 1] Camera Movement
  (Default|BasicMovementForward (Variables|References|GetCameraMovementRef) ActionValue))

(event Input|EnhancedActionEvents|EnhancedInputActionIA_MoveRight
  (params (ActionValue :type Float%20%28double-precision%29) (ElapsedSeconds :type Float%20%28double-precision%29) (TriggeredSeconds :type Float%20%28double-precision%29) (InputAction :type Input%20Action%20Object%20Reference :default "/Game/RTSGAME/Core/Settings/Input/Actions/IA_MoveRight.IA_MoveRight"))
  ;[1 1 1] Camera Movement
  (Default|BasicMovementRight (Variables|References|GetCameraMovementRef) ActionValue))

(event Input|EnhancedActionEvents|EnhancedInputActionIA_ZoomIn
  (params (ActionValue :type Boolean) (ElapsedSeconds :type Float%20%28double-precision%29) (TriggeredSeconds :type Float%20%28double-precision%29) (InputAction :type Input%20Action%20Object%20Reference :default "/Game/RTSGAME/Core/Settings/Input/Actions/IA_ZoomIn.IA_ZoomIn"))
  ;[1 1 1] Camera Zoom
  (Default|Zoomin (Variables|References|GetCameraMovementRef)))

(event Input|EnhancedActionEvents|EnhancedInputActionIA_ZoomOut
  (params (ActionValue :type Boolean) (ElapsedSeconds :type Float%20%28double-precision%29) (TriggeredSeconds :type Float%20%28double-precision%29) (InputAction :type Input%20Action%20Object%20Reference :default "/Game/RTSGAME/Core/Settings/Input/Actions/IA_ZoomOut.IA_ZoomOut"))
  ;[1 1 1] Camera Zoom
  (Default|ZoomOut (Variables|References|GetCameraMovementRef)))

(event Input|EnhancedActionEvents|EnhancedInputActionIA_CameraPan
  (params (ActionValue :type Boolean) (ElapsedSeconds :type Float%20%28double-precision%29) (TriggeredSeconds :type Float%20%28double-precision%29) (InputAction :type Input%20Action%20Object%20Reference :default "/Game/RTSGAME/Core/Settings/Input/Actions/IA_CameraPan.IA_CameraPan"))
  (bind _cameramovementref (Variables|References|GetCameraMovementRef))
  ;[1 1 1] Camera Pan
  (:Triggered
    (Variables|/Game/RTSGAME/Core/Player/BPC_PawnMovement.BPC_PawnMovement_C|SetbDisableEdgeScroll _cameramovementref true)
    (Utilities|FlowControl|Gate false) ; enters at Open
  )
  (:Completed
    (Variables|/Game/RTSGAME/Core/Player/BPC_PawnMovement.BPC_PawnMovement_C|SetbDisableEdgeScroll _cameramovementref false)
    (Utilities|FlowControl|Gate false) ; enters at Close
  ))

(event EventBeginPlay
  (bind _returnvalue (PlayerController|LocalPlayerSubsystems|GetEnhancedInputLocalPlayerSubsystem))
  (Utilities|FlowControl|Sequence
    (:then_0
      (Variables|Default|SetbShowMouseCursor true)
      (bind _asbp_camera_pawn (Utilities|Casting|CastToBP_CameraPawn (Game|Player|GetPlayerPawn 0)))
      (bind _output_get (Variables|References|SetCameraPawnRef _asbp_camera_pawn))
      (Variables|References|SetCameraMovementRef (Variables|/Game/RTSGAME/Core/Player/BP_CameraPawn.BP_CameraPawn_C|GetBPC_PawnMovement _output_get))
      (Utilities|IsValid _returnvalue
        (:Is%20Valid
          (Input|AddMappingContext _returnvalue "/Game/RTSGAME/Core/Settings/Input/IMC_Input.IMC_Input" 0 "(bIgnoreAllPressedKeysUntilRelease=True,bForceImmediately=False,bNotifyUserSettings=False)"))))
    (:then_1
      (bind _returnvalue_2 (UserInterface|CreateWidget "/Game/RTSGAME/Core/UI/Widgets/WBP_MainUI.WBP_MainUI_C" self))
      (bind _output_get_2 (Variables|References|SetMainWidgetRef _returnvalue_2))
      (UserInterface|Viewport|AddtoViewport _output_get_2 0)
      (Input|SetInputModeGameandUI self _output_get_2 "LockInFullscreen" false false))
    (:then_2
      (bind _outactors (Actor|GetAllActorsOfClass "/Game/RTSGAME/Core/Units/ParentPlayableUnitClass.ParentPlayableUnitClass_C"))
      (for _array_element _outactors
        (Default|MakeAnIcon _array_element)
        (Utilities|FlowControl|Delay 0.1)))))

(event EventAddUnittoUnitsArea
  (params (UnitWidget :type User%20Widget%20Object%20Reference))
  (Widget|Panel|AddChild (Variables|/Game/RTSGAME/Core/UI/Widgets/WidgetSubMenus/WBP_UnitsArea.WBP_UnitsArea_C|GetSB_Units (Variables|/Game/RTSGAME/Core/UI/Widgets/WBP_MainUI.WBP_MainUI_C|GetWBP_UnitsArea (Variables|References|GetMainWidgetRef))) UnitWidget))

(event EventUnitLay
  (bind _units (Class|BPIInteractions|GrabSelectedUnits(Message) (HUD|GetHUD)))
  (for _array_element _units
    (Class|BPIInteractions|UnitLay(Message) _array_element)))

(event EventUpdateGameSpeed
  (params (NewSpeedMultiplier :type Float%20%28double-precision%29))
  (Class|BPIGameTime|UpdateGameSpeed(Message) (Game|GetGameState) NewSpeedMultiplier))

(event EventSetDateTime
  (params (DateTimeStruct :type Date%20Time%20Structure))
  (Class|BPIGameTime|SetDateTime(Message) (Variables|References|GetMainWidgetRef) DateTimeStruct))

(event EventSetGameSpeedInt
  (params (GameSpeed :type Float%20%28double-precision%29))
  (Class|BPIGameTime|SetGameSpeedInt(Message) (Variables|References|GetMainWidgetRef) GameSpeed))

(event EventSetCameraTimeDilation
  (params (SpeedSetting :type Integer))
  (Default|SetCameraTimeDilation (Variables|References|GetCameraPawnRef) SpeedSetting))

(event EventTick
  (params (DeltaSeconds :type Float%20%28single-precision%29))
  (if (Variables|Default|GetbIsLMBPressed)
    (Class|BPISelection|MarqueeHeld(Message) (HUD|GetHUD))))

(event EventUnitRun
  (bind _units (Class|BPIInteractions|GrabSelectedUnits(Message) (HUD|GetHUD)))
  (for _array_element _units
    (Class|BPIInteractions|UnitRun(Message) _array_element)))

(event EventUnitWalk
  (bind _units (Class|BPIInteractions|GrabSelectedUnits(Message) (HUD|GetHUD)))
  (for _array_element _units
    (Class|BPIInteractions|UnitWalk(Message) _array_element)))

(event EventUnitCrouch
  (bind _units (Class|BPIInteractions|GrabSelectedUnits(Message) (HUD|GetHUD)))
  (for _array_element _units
    (Class|BPIInteractions|UnitCrouch(Message) _array_element)))

(event Input|MouseEvents|MouseY
  (params (AxisValue :type Float%20%28single-precision%29))
  (bind _cameramovementref (Variables|References|GetCameraMovementRef))
  ;[1 1 1] Camera Pan
  (Utilities|FlowControl|Sequence
    (:then_0
      (Utilities|FlowControl|Gate false
        (:Exit
          (Default|PanCameraUpDown _cameramovementref (* AxisValue (Variables|Camera|Settings|GetPanSensitivity)))
          (Default|PanCameraRightLeft _cameramovementref (* (stale Input|MouseEvents|MouseX AxisValue) (Variables|Camera|Settings|GetPanSensitivity))))))
    (:then_1
      ;[1 1 1] EdgeScroll
      (Default|EdgeScroll (Variables|References|GetCameraMovementRef)))))

(event Input|MouseEvents|MouseX
  (params (AxisValue :type Float%20%28single-precision%29))
  (bind _cameramovementref (Variables|References|GetCameraMovementRef))
  ;[1 1 1] Camera Pan
  (Utilities|FlowControl|Sequence
    (:then_0
      (Utilities|FlowControl|Gate false
        (:Exit
          (Default|PanCameraUpDown _cameramovementref (* (stale Input|MouseEvents|MouseY AxisValue) (Variables|Camera|Settings|GetPanSensitivity)))
          (Default|PanCameraRightLeft _cameramovementref (* AxisValue (Variables|Camera|Settings|GetPanSensitivity))))))
    (:then_1
      ;[1 1 1] EdgeScroll
      (Default|EdgeScroll (Variables|References|GetCameraMovementRef)))))

(event Input|MouseEvents|LeftMouseButton
  (params (Key :type Key%20Structure :default "None"))
  (bind _returnvalue (HUD|GetHUD))
  (:Pressed
    (Variables|Default|SetbIsLMBPressed true)
    (Class|BPISelection|MarqueePressed(Message) _returnvalue))
  (:Released
    (Variables|Default|SetbIsLMBPressed false)
    (Class|BPISelection|MarqueeReleased(Message) _returnvalue)))

(event Input|MouseEvents|RightMouseButton
  (params (Key :type Key%20Structure :default "None"))
  (:Pressed
    (bind _output_get (Variables|Default|SetRightClickLocation (.Location (Collision|BreakHitResult (.HitResult (Game|Player|GetHitResultUnderCursorbyChannel "TraceTypeQuery1" true))))))
    (bind _units (Class|BPIInteractions|GrabSelectedUnits(Message) (HUD|GetHUD)))
    (for _array_element _units
      (Class|BPIInteractions|UnitMoveCommand(Message) _array_element _output_get))
    (Niagara|SpawnSystematLocation "/Game/Cursor/FX_Cursor.FX_Cursor" _output_get)))

(fn ConstructionScript)

(fn GetUnitIconWidget
  (return 0))

(fn GetUnitLocomotion
  (return "NewEnumerator0"))

(fn GrabSelectedUnits
  (return 0))