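; RTS player camera pawn that holds a target height above the terrain and supports spring-arm zoom.
; BPCPawnMovement is initialized on BeginPlay, while each tick a downward trace drives swept vertical offsets toward the target height.
; SetArmLength maps zoom amount to arm length through a float curve.
; SetCameraTimeDilation sets inverse custom time dilation per speed setting, including a huge factor for setting zero, apparently offsetting game speed.
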(event Custom|SetCameraTimeDilation
  (params (SpeedSetting :type Integer))
  (switch int SpeedSetting
    (:Default
      (Variables|Default|SetCustomTimeDilation 1.0 :!label _label))
    (:0
      (Variables|Default|SetCustomTimeDilation 1e+06))
    (:1
      (Variables|Default|SetCustomTimeDilation 4.0))
    (:2
      (Variables|Default|SetCustomTimeDilation 2.0))
    (:3
      (goto _label))
    (:4
      (Variables|Default|SetCustomTimeDilation 0.5))
    (:5
      (Variables|Default|SetCustomTimeDilation 0.25))))

(event EventBeginPlay
  (Default|InitComponent (Variables|Default|GetBPC_PawnMovement)))

(event Collision|EventActorBeginOverlap
  (params (OtherActor :type Actor%20Object%20Reference)))

(event EventTick
  (params (DeltaSeconds :type Float%20%28single-precision%29))
  (Camera|Height|AdjustCameraHeight))

(fn ConstructionScript)

(fn SetArmLength
  (params (InZoomAmount :type Float%20%28double-precision%29))
  (bind _curvezoomoutlenght (Variables|Camera|Zoom|GetCurveZoomOutLenght)
    (:then
      (Variables|/Script/Engine.SpringArmComponent|SetTargetArmLength (Variables|Default|GetSpringArm) (Math|Curves|GetFloatValue _curvezoomoutlenght InZoomAmount)))
    (:else
      _))
  (return))

(fn AdjustCameraHeight
  (bind _returnvalue (Transformation|GetActorLocation))
  (bind _outhit (Collision|LineTraceByChannel _returnvalue (- _returnvalue "0.000000,0.000000,10000.000000") "TraceTypeQuery3" false 0 "None"))
  (bind _output_get (LocalVariables|SetDistanceLocal (Math|Vector|VectorLength (- (.ImpactPoint (Collision|BreakHitResult _outhit)) (Transformation|GetActorLocation)))))
  (if (Math|Float|NearlyEqual(Float) _output_get (Variables|Default|GetTargetPawnHeight) 0.05)
    (return)
    (else
      ;[1 1 1] Too High, adjust down
      (if (> (LocalVariables|GetDistanceLocal) (Variables|Default|GetTargetPawnHeight))
        (Transformation|AddActorLocalOffset (Math|Vector|MakeVector 0.0 0.0 (- (Variables|Default|GetTargetPawnHeight) (LocalVariables|GetDistanceLocal))) true false)
        (return)
        (else
          (Transformation|AddActorLocalOffset (Math|Vector|MakeVector 0.0 0.0 (+ (- (Variables|Default|GetTargetPawnHeight) (LocalVariables|GetDistanceLocal)) 5.0)) true false))))))