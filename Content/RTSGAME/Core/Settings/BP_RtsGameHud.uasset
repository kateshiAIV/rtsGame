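; RTS HUD Blueprint that draws the marquee selection box and maintains the list of selected units.
; Marquee press, hold and release events track the mouse rectangle from player controller 0.
; While dragging, DrawHUD renders the box, selects actors inside and deselects units outside through message calls.
; SelectSingleUnit adds individual units and GrabSelectedUnits exposes the list, while the unit-state and icon getters are empty stubs.
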(event EventSelectSingleUnit
  (params (Unit :type Actor%20Object%20Reference))
  (Class|BPISelection|SelectUnit(Message) Unit)
  (Utilities|Array|AddUnique (Variables|Default|GetSelectedUnits) Unit))

(event EventMarqueeReleased
  (Variables|Default|SetbIsDrawing false))

(event EventMarqueeHeld
  (bind _returnvalue (Game|GetPlayerController 0))
  (bind (_locationx _locationy) (Game|Player|GetMousePosition _returnvalue))
  ;[1 1 1] Held  Selection
  (Variables|Default|SetCurrentMousePosition (Math|Vector2D|MakeVector2D _locationx _locationy)))

(event EventMarqueePressed
  (bind _returnvalue (Game|GetPlayerController 0))
  (bind (_locationx _locationy) (Game|Player|GetMousePosition _returnvalue))
  ;[1 1 1] Start Selection
  (Variables|Default|SetbIsDrawing true)
  (Variables|Default|SetStartMousePosition (Math|Vector2D|MakeVector2D _locationx _locationy))
  (Variables|Default|SetCurrentMousePosition (Math|Vector2D|MakeVector2D _locationx _locationy)))

(event EventDrawHUD
  (params (SizeX :type Integer) (SizeY :type Integer))
  (bind _startmouseposition (Variables|Default|GetStartMousePosition))
  (bind _currentmouseposition (Variables|Default|GetCurrentMousePosition))
  (bind _startmouseposition_2 (Variables|Default|GetStartMousePosition))
  (if (Variables|Default|GetbIsDrawing)
    (HUD|DrawRect "(R=0.000000,G=0.878946,B=1.000000,A=0.100000)" (.x _startmouseposition) (.y _startmouseposition) (- (.x _currentmouseposition) (.x _startmouseposition_2)) (- (.y _currentmouseposition) (.y _startmouseposition_2)))
    (bind _output_get (Variables|Default|SetActorsInRect (Class|HUD|GetActorsinSelectionRectangle "/Script/Engine.Actor" (Variables|Default|GetStartMousePosition) (Variables|Default|GetCurrentMousePosition) false false)))
    (for _array_element _output_get
      (Class|BPISelection|SelectUnit(Message) _array_element)
      (Utilities|Array|AddUnique (Variables|Default|GetSelectedUnits) _array_element))
    (for _array_element_2 (Variables|Default|GetSelectedUnits)
      (if (== (Utilities|Array|FindItem (Variables|Default|GetActorsInRect) _array_element_2) -1)
        (Class|BPISelection|DeselectUnit(Message) _array_element_2)
        (Utilities|Array|RemoveItem (Variables|Default|GetSelectedUnits) _array_element_2)))))

(fn ConstructionScript)

(fn GetIsUnitCrouching
  (return false))

(fn GetIsUnitLaying
  (return false))

(fn GetIsUnitRunning
  (return false))

(fn GetIsUnitWalking
  (return false))

(fn GetUnitIconWidget
  (return 0))

(fn GrabSelectedUnits
  (return (Variables|Default|GetSelectedUnits)))