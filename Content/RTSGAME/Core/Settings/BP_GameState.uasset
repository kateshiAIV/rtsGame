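; Game state for the RTS that runs the in-game clock and calendar at an adjustable game speed.
; While speed is nonzero, Tick advances game time, derives time and date with day, month and year rollover, and debug-prints them.
; It sends the time to the BP_SunRotation actor and a DateTime struct to the player controller via messages.
; Speed changes scale the default speed and fire a game-speed event.
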(event Custom|CalculateTime
  (params (DeltaTime :type Float%20%28double-precision%29))
  (Variables|GameSpeed|Settings|SetGameTime (.OutGameTime (CallFunction|CalculateGameTime DeltaTime (Variables|GameSpeed|Settings|GetGameSpeed) (Variables|GameSpeed|Settings|GetGameTime))))
  (Variables|Calendar|SetDayCounter (.DayCounter (CallFunction|CalculateGameTime DeltaTime (Variables|GameSpeed|Settings|GetGameSpeed) (Variables|GameSpeed|Settings|GetGameTime)))))

(event Custom|SetClockCalendar
  (bind (_year _month _day _hours _minutes _seconds) (CallFunction|UpdateClockCalendar))
  (CallFunction|SetDateTimeSruct _year _month _day _hours _minutes _seconds)
  (CallFunction|DebugPrintGameTime _year _month _day _hours _minutes _seconds))

(event Custom|PassGameTime
  (bind _sunactorref (Variables|References|GetSunActorRef)
    (:then
      (Class|BPIGameTime|SetGameTime(Message) _sunactorref (Variables|GameSpeed|Settings|GetGameTime)))
    (:else)))

(event Custom|GetSunRotationActor
  (bind _returnvalue (Actor|GetActorOfClass "/Game/RTSGAME/Core/Actors/GameTime/BP_SunRotation.BP_SunRotation_C"))
  (Variables|References|SetSunActorRef _returnvalue))

(event Custom|PassGameTimeStruct
  (Class|BPIGameTime|SetDateTime(Message) (Game|GetPlayerController 0) (Variables|GameSpeed|Settings|GetDateTimeStruct)))

(event EventBeginPlay
  (GameSpeed|Settings|SetInitialGameTime)
  (CallFunction|GetSunRotationActor))

(event EventTick
  (params (DeltaSeconds :type Float%20%28single-precision%29))
  (if (!= (Variables|GameSpeed|Settings|GetGameSpeed) 0.0)
    (CallFunction|CalculateTime DeltaSeconds)
    (CallFunction|SetClockCalendar)
    (CallFunction|PassGameTime)
    (CallFunction|PassGameTimeStruct)))

(event EventUpdateGameSpeed
  (params (NewSpeedMultiplier :type Float%20%28double-precision%29))
  (bind _output_get (Variables|GameSpeed|Settings|SetGameSpeed (* NewSpeedMultiplier (Variables|GameSpeed|Settings|GetDefaultGameSpeed))))
  (Default|CallOnGameSpeedControl _output_get))

(fn ConstructionScript)

(fn SetInitialGameTime
  (Variables|GameSpeed|Settings|SetGameTime (+ (Math|Conversions|ToFloat(Integer) (Variables|Clock|GetHours)) (/ (Variables|Clock|GetMinutes) (LocalVariables|GetBLocal)) (/ (Variables|Clock|GetSeconds) 3.6e+03))))

(fn UpdateClockCalendar
  (bind _gametime (Variables|GameSpeed|Settings|GetGameTime))
  (bind _returnvalue (* _gametime 3.6e+03))
  (bind (_remainder _returnvalue_2) (Math|Float|Division(WholeandRemainder) _returnvalue 6e+01))
  (bind _returnvalue_3 (Math|Conversions|ToFloat(Integer) _returnvalue_2))
  (bind (_remainder_2 _returnvalue_4) (Math|Float|Division(WholeandRemainder) _returnvalue_3 6e+01))
  ;[1 1 1] Set seconds
  (Variables|Clock|SetSeconds (Math|Float|Floor _remainder))
  ;[1 1 1] Set minutes
  (Variables|Clock|SetMinutes (Math|Float|Floor _remainder_2))
  ;[1 1 1] Set hours
  (Variables|Clock|SetHours (Math|Float|Floor (.Remainder (Math|Float|Division(WholeandRemainder) (Math|Conversions|ToFloat(Integer) _returnvalue_4) 24.0))))
  ;[1 1 1] Calendar
  (bind _output_get (Variables|Calendar|SetDay (+ (Variables|Calendar|GetDayCounter) (Variables|Calendar|GetDay))))
  (if (> _output_get (Class|KismetMathLibrary|DaysinMonth (Variables|Calendar|GetYear) (Variables|Calendar|GetMonth)))
    (Variables|Calendar|SetDay 1)
    (Variables|Calendar|SetMonth (+ (Variables|Calendar|GetMonth) 1)))
  (if (> (Variables|Calendar|GetMonth) 12)
    (Variables|Calendar|SetMonth 1)
    (Variables|Calendar|SetYear (+ (Variables|Calendar|GetYear) 1)))
  (return (Variables|Calendar|GetYear) (Variables|Calendar|GetMonth) (Variables|Calendar|GetDay) (Variables|Clock|GetHours) (Variables|Clock|GetMinutes) (Variables|Clock|GetSeconds)))

(fn SetDateTimeSruct
  (params (Year :type Integer%20%28by%20ref%29) (Month :type Integer%20%28by%20ref%29) (Day :type Integer%20%28by%20ref%29) (Hour :type Integer%20%28by%20ref%29) (Minute :type Integer%20%28by%20ref%29) (Second :type Integer%20%28by%20ref%29))
  (Variables|GameSpeed|Settings|SetDateTimeStruct (Math|DateTime|MakeDateTime Year Month Day Hour Minute Second)))

(fn DebugPrintGameTime
  (params (Year :type Integer%20%28by%20ref%29) (Month :type Integer%20%28by%20ref%29) (Day :type Integer%20%28by%20ref%29) (Hour :type Integer%20%28by%20ref%29) (Minutes :type Integer%20%28by%20ref%29) (Seconds :type Integer%20%28by%20ref%29))
  (Development|PrintString (Utilities|String|Append (Utilities|String|ToString(Integer) Hour) ":" (Utilities|String|ToString(Integer) Minutes) ":" (Utilities|String|ToString(Integer) Seconds) "     " (Utilities|String|ToString(Integer) Day) "/" (Utilities|String|ToString(Integer) Month) "/" (Utilities|String|ToString(Integer) Year)) true false "(R=0.000000,G=0.660000,B=1.000000,A=1.000000)" 0.01))